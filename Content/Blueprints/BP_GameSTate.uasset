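; Game state Blueprint that runs the round flow of a falling-pom matching puzzle.
; On BeginPlay it caches the game instance, spawns the initial row, then spawns the first pom after a short delay.
; When a pom stops, a delayed loop clears poms and moves the rest down until nothing clears, then spawns the next one, using game instance timings.
; Lose and Restart only toggle the game-over flag.
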(event Custom|Handle%20Pom%20Stopped
  (bind _game_instance (Variables|Default|GetGame%20Instance))
  (bind _countcleared (Class|MyGameState|ClearPoms :!label _label))
  (Utilities|FlowControl|Delay (Variables|/Game/Blueprints/BP_GameInstance.BP_GameInstance_C|GetPom%20Fade%20Time _game_instance))
  (if (> _countcleared 0)
    (Class|MyGameState|MovePomsDown)
    (Utilities|FlowControl|Delay (Variables|/Game/Blueprints/BP_GameInstance.BP_GameInstance_C|GetDelay%20After%20Fade _game_instance))
    (goto _label)
    (else
      (Class|MyGameState|SpawnNewPom))))

(event EventRestart
  (Variables|Default|Setm_gameOver false))

(event EventLose
  (Variables|Default|Setm_gameOver true))

(event EventBeginPlay
  (Variables|Default|SetGame%20Instance (.AsBP%20Game%20Instance (Utilities|Casting|CastToBP_GameInstance (Game|GetGameInstance))))
  (Class|MyGameState|SpawnInitialRow)
  (Utilities|FlowControl|Delay 0.2)
  (Class|MyGameState|SpawnNewPom))

(fn ConstructionScript)