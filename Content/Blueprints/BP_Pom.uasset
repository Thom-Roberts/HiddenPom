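; BP_Pom is a colored cube piece for a grid-based puzzle game, taking a random red, yellow, green or blue material on spawn.
; BottomOffset overlaps with anything but its own cube raise overlap calls, and a line trace from that point tests whether it can move sideways.
; On becoming inactive, it records its color and grid cell in BP_GameState.
; A timeline scaled by the GameInstance fade time fades its dynamic material, then destroys it.
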(event OnComponentEndOverlap(BottomOffset)
  (params (OverlappedComponent :type Primitive%20Component%20Object%20Reference) (OtherActor :type Actor%20Object%20Reference) (OtherComp :type Primitive%20Component%20Object%20Reference) (OtherBodyIndex :type Integer))
  (if (!= OtherComp (Variables|Default|GetCube))
    (Default|CallOverlapExit)))

(event OnComponentBeginOverlap(BottomOffset)
  (params (OverlappedComponent :type Primitive%20Component%20Object%20Reference) (OtherActor :type Actor%20Object%20Reference) (OtherComp :type Primitive%20Component%20Object%20Reference) (OtherBodyIndex :type Integer) (bFromSweep :type Boolean) (SweepResult :type Hit%20Result%20Structure%20%28by%20ref%29))
  (if (!= OtherComp (Variables|Default|GetCube)) ; Solves issue where item was overlapping with itself
    (Default|CallOverlapOccurred)))

(event EventBecomeInactive
  (bind (_row _column) (Utilities|GetPomIndexPositionforState))
  (Class|MyGameState|SetPomColorPosition (.AsBP%20Game%20State (Utilities|Casting|CastToBP_GameState (Game|GetGameState))) _row _column (Variables|Default|GetColor) self))

(event EventSetPomColor
  (params (color :type PomColor%20Enum :default "None"))
  (bind _output_get (Variables|Default|SetColor color))
  (bind _material (CallFunction|GetMaterialfromPomColor _output_get))
  (CallFunction|SetCubeMaterial _material))

(event EventBeginPlay
  (CallFunction|GenerateandSetPomColor)
  (Variables|Default|SetGame%20Instance (.AsBP%20Game%20Instance (Utilities|Casting|CastToBP_GameInstance (Game|GetGameInstance)))))

(event EventFadeThenDestroy
  (Components|Timeline|SetPlayRate (Variables|Default|GetFade%20Material%20Timeline) (/ 1.0 (Variables|/Game/Blueprints/BP_GameInstance.BP_GameInstance_C|GetPom%20Fade%20Time (Variables|Default|GetGame%20Instance))))
  (bind _fade (Timeline|Fade%20Material%20Timeline PlayFromStart)
    (:Update
      (Rendering|Material|SetScalarParameterValue (Variables|Default|GetCube%20Dynamic%20Material) "Fade Amount" _fade :!class /Script/Engine.MaterialInstanceDynamic))
    (:Finished
      (Actor|DestroyActor))))

(fn ConstructionScript)

(fn GenerateandSetPomColor
  (bind _output_get (LocalVariables|SetRandom%20Num (Math|Random|RandomIntegerinRange 0 (- (Utilities|Array|Length (Variables|Default|GetMaterials)) 1))))
  (CallFunction|SetCubeMaterial (Utilities|Array|Get(acopy) (Variables|Default|GetMaterials) _output_get))
  (switch int (LocalVariables|GetRandom%20Num) ; Reliant on Materials being in Red, Yellow, Green, Blue order
    (:0
      (Variables|Default|SetColor "Red"))
    (:1
      (Variables|Default|SetColor "Yellow"))
    (:2
      (Variables|Default|SetColor "Green"))
    (:3
      (Variables|Default|SetColor "Blue")))
  (return))

(fn TestifCanMoveHorizontal
  (params (Direction :type Float%20%28single-precision%29) (Actors%20To%20Ignore :type Array%20of%20Actor%20Object%20References))
  (bind _bottom_offset (Variables|Default|GetBottom%20Offset))
  (bind _returnvalue (Transformation|GetWorldLocation _bottom_offset))
  (bind _output_get (LocalVariables|SetCastStart (Math|Vector|MakeVector (.x _returnvalue) (.y _returnvalue) (+ (.z _returnvalue) 25.0))))
  (bind _returnvalue_2 (Collision|LineTraceByChannel _output_get (Math|Vector|MakeVector (.x (LocalVariables|GetCastStart)) (+ (* Direction (Variables|Default|GetMove%20Distance)) (.y (LocalVariables|GetCastStart))) (.z (LocalVariables|GetCastStart))) "TraceTypeQuery1" false Actors%20To%20Ignore "ForDuration"))
  (return (not _returnvalue_2)))

(fn GetMaterialfromPomColor
  (params (Color :type PomColor%20Enum :default "None"))
  (switch Utilities|FlowControl|Switch|SwitchonPomColor Color
    (:Red
      (LocalVariables|SetColor%20Index 0))
    (:Yellow
      (LocalVariables|SetColor%20Index 1))
    (:Green
      (LocalVariables|SetColor%20Index 2))
    (:Blue
      (LocalVariables|SetColor%20Index 3)))
  (return (Utilities|Array|Get(acopy) (Variables|Default|GetMaterials) (LocalVariables|GetColor%20Index))))

(fn SetCubeMaterial
  (params (Material :type Material%20Instance%20Object%20Reference))
  (bind _cube (Variables|Default|GetCube))
  (Rendering|Material|SetMaterial _cube 0 Material)
  (bind _returnvalue (Rendering|Material|CreateDynamicMaterialInstance _cube 0 Material "None" :!class /Script/Engine.PrimitiveComponent))
  (Variables|Default|SetCube%20Dynamic%20Material _returnvalue))