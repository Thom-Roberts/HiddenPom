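; BP_DoublePom is the falling pair of Poms that the player controls in a grid-stepped drop puzzle.
; While it is the player's CurrentPom, Tick steps it down on a timer, shortened by holding down, using a swept move gated by the bottom Pom's overlap events.
; Sideways moves teleport the pair after both child Poms pass their checks.
; A failed drop deactivates both Poms and can notify BP_GameState.
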(event Custom|Try%20Move%20Horizontal
  (params (Direction :type Float%20%28single-precision%29))
  (bind _can_move (CallFunction|TestifBothPomsCanMove Direction))
  (if _can_move
    (Utilities|MoveActors Direction)))

(event Custom|Increase%20Drop%20Speed
  (Variables|Default|SetHolding%20Down true))

(event Custom|Reset%20Drop%20Speed
  (Variables|Default|SetHolding%20Down false))

(event Custom|Exited%20Collision
  (Variables|Default|SetCan%20Move%20Down true))

(event Custom|Collision%20on%20Bottom%20Pom
  (Variables|Default|SetCan%20Move%20Down false))

(event EventBeginPlay
  (Variables|Components|SetTop%20Pom%20Actor (Utilities|ExtractPomClass (Variables|Default|GetTop%20Pom)))
  (bind _output_get (Variables|Components|SetBottom%20Pom%20Actor (Utilities|ExtractPomClass (Variables|Default|GetBottom%20Pom))))
  (EventDispatchers|BindEventtoOverlapOccurred _output_get (delegate Custom|Collision%20on%20Bottom%20Pom))
  (EventDispatchers|BindEventtoOverlapExit _output_get (delegate Custom|Exited%20Collision))
  (Transformation|SetActorRotation "0, 0, 0") ; Temporary fix for spawn setting rotation for some reason
  (Variables|Default|SetPlayer%20Pawn (.AsBP%20Player (Utilities|Casting|CastToBP_Player (Game|Player|GetPlayerPawn 0)))))

(event EventBecomeInactive
  (Variables|/Script/Pom.PlayerBase|SetcurrentPom (Variables|Default|GetPlayer%20Pawn) 0)
  (Class|PomBase|BecomeInactive (Variables|Components|GetTop%20Pom%20Actor))
  (Class|PomBase|BecomeInactive (Variables|Components|GetBottom%20Pom%20Actor))
  (Variables|Default|SetCan%20Move%20Down false)
  (if (Variables|Default|Getm_shouldTriggerOverlaps)
    (Default|HandlePomStopped (.AsBP%20Game%20State (Utilities|Casting|CastToBP_GameState (Game|GetGameState))))))

(event EventTick
  (params (DeltaSeconds :type Float%20%28single-precision%29))
  (if (== (Variables|/Script/Pom.PlayerBase|GetcurrentPom (Variables|Default|GetPlayer%20Pawn)) self) ; If we're inactive, break early
    (bind _successful (CallFunction|TryMoveDown DeltaSeconds))
    (if (not _successful) ; Attempted to move, but failed?
      (Class|PomBase|BecomeInactive))))

(fn ConstructionScript)

(fn TestifBothPomsCanMove
  (params (Direction :type Float%20%28single-precision%29))
  (Utilities|FlowControl|Sequence
    (:then_0
      (bind _no_collision (Default|TestifCanMoveHorizontal (Variables|Components|GetTop%20Pom%20Actor) Direction (Utilities|Array|MakeArray (Variables|Components|GetBottom%20Pom%20Actor)))))
    (:then_1
      (bind _no_collision_2 (Default|TestifCanMoveHorizontal (Variables|Components|GetBottom%20Pom%20Actor) Direction (Utilities|Array|MakeArray (Variables|Components|GetTop%20Pom%20Actor))))
      (return (and _no_collision _no_collision_2)))))

(fn TryMoveDown
  (params (Delta%20Seconds :type Float%20%28single-precision%29))
  (bind _output_get (Variables|Default|SetCurrent%20Tick%20Delay (+ Delta%20Seconds (Variables|Default|GetCurrent%20Tick%20Delay))))
  (if (|TimeExpired _output_get) ; Should we attempt the move?
    (Variables|Default|SetCurrent%20Tick%20Delay 0.0) ; Start trying to move
    (if (Variables|Default|GetCan%20Move%20Down)
      (bind _moved (Utilities|MoveActorsDown)
        (:Out
          (LocalVariables|SetReturnVal _moved)))
      (else
        (LocalVariables|SetReturnVal false)))
    (else
      (LocalVariables|SetReturnVal true) ; Return Successful if no need to move
    ))
  (return (LocalVariables|GetReturnVal)))