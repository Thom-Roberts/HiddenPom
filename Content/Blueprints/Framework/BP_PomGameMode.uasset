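; BP_PomGameMode is a game mode Blueprint that holds the rules for turning a CP value into attack rows, defend rows and special-action eligibility.
; Attack and defend rows come from dividing CP by separate per-row variables, with defense clamped to at least one row.
; A special action is allowed once CP reaches the PointsToDoAction threshold.
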(fn ConstructionScript)

(fn CalculateAttackRows
  (params (CP :type Integer))
  (return (/ CP (Variables|Default|GetAttack%20CP%20per%20row))))

(fn CalculateDefendRows
  (params (CP :type Integer))
  (return (Math|Integer|Max(Integer) (/ CP (Variables|Default|GetDefense%20CP%20per%20row)) 1)))

(fn CanDoSpecialAction
  (params (CP :type Integer))
  (return (>= CP (Variables|Default|GetPoints%20To%20Do%20Action))))