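; BP_GameState runs the core loop and scoring of a Pom-clearing puzzle game.
; BeginPlay shows the score widget, spawns initial rows, then sets up active and preview Poms.
; When a Pom stops, it repeatedly clears Poms, adding escalating score and moving Poms down after the fade, until none clear.
; It then resets the bonus and promotes the preview Pom after a delay, flagging game over if that fails.
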(event Custom|Handle%20Pom%20Stopped
  (bind _countcleared (Class|MyGameState|ClearPoms :!label _label))
  (if (> _countcleared 0) ; We only need to delay if we're actually clearing poms
    (|IncreaseScoreandMovepomsdown)
    (goto _label)
    (else
      (Class|MyGameState|ResetScoreBonus)
      (Utilities|FlowControl|Delay (Variables|/Game/Blueprints/Framework/BP_GameInstance.BP_GameInstance_C|GetDelay%20After%20Fade (Variables|Default|GetGame%20Instance)))
      (bind _success (Class|MyGameState|SetActivePom (Variables|Default|GetPreviewPom)))
      (if _success
        (bind _returnvalue (Class|MyGameState|SpawnNewPominPreviewPosition))
        (Variables|Default|SetPreviewPom _returnvalue)
        (else
          (Class|MyGameState|Lose))))))

(event EventRestart
  (Variables|Default|Setm_gameOver false))

(event EventLose
  (Variables|Default|Setm_gameOver true))

(event EventBeginPlay
  (Utilities|FlowControl|Sequence
    (:then_0
      (bind _returnvalue (UserInterface|CreateWidget "/Game/Blueprints/Widgets/BPW_Score.BPW_Score_C" (Game|GetPlayerController 0)))
      (UserInterface|Viewport|AddtoViewport _returnvalue 0))
    (:then_1
      (Variables|Default|SetGame%20Instance (.AsBP%20Game%20Instance (Utilities|Casting|CastToBP_GameInstance (Game|GetGameInstance))))
      (Class|MyGameState|SpawnInitialRows)
      (Utilities|FlowControl|Delay 0.2)
      (bind _returnvalue_2 (Class|MyGameState|SpawnNewPominPreviewPosition))
      (Class|MyGameState|SetActivePom _returnvalue_2)
      (bind _returnvalue_3 (Class|MyGameState|SpawnNewPominPreviewPosition))
      (Variables|Default|SetPreviewPom _returnvalue_3))))

(fn ConstructionScript)